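; BP_baseEnemy is a base enemy character that periodically turns toward the player and teleports.
; Timed BeginPlay loops re-aim it and trace to the player, moving it to a random reachable point around an "MO"-tagged actor on a non-zero hit location.
; Damage goes to a health component and can launch it upward; fragment hits show a timed Stun visual.
; The navmesh flee-from-player logic is disconnected from its overlap event.
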(event OnComponentBeginOverlap(Distance_collision)
  (params (OverlappedComponent :type Primitive%20Component%20Object%20Reference) (OtherActor :type Actor%20Object%20Reference) (OtherComp :type Primitive%20Component%20Object%20Reference) (OtherBodyIndex :type Integer) (bFromSweep :type Boolean) (SweepResult :type Hit%20Result%20Structure%20%28by%20ref%29))
  ;[0.15 0.15 0.15 0.5] Uses Distance_collision to flee from Player
)

(event EventBeginPlay
  (bind _returnvalue (Transformation|GetActorLocation))
  (bind _outactors (Actor|GetAllActorsOfClasswithTag "/Script/Engine.Actor" "MO"))
  (bind _asbp_first_person_character (Utilities|Casting|CastToBP_FirstPersonCharacter (Game|GetPlayerCharacter 0)))
  (bind _output_get (Variables|Default|SetAs%20BP%20First%20Person%20Character _asbp_first_person_character))
  (Utilities|FlowControl|Sequence
    (:then_0
      ;[0.15 0.15 0.15 0.5] DL to rotate enemy toward Player
      ;;[0.15 0 0 0.5] change to be conditional when player is in zone
      (Utilities|FlowControl|Delay 2.0 :!label _label)
      (Transformation|SetActorRotation (Math|Rotator|MakeRotator 0.0 (.pitch (Math|Rotator|FindLookatRotation _returnvalue (Transformation|GetActorLocation _output_get))) (.yaw (Math|Rotator|FindLookatRotation _returnvalue (Transformation|GetActorLocation _output_get)))))
      (goto _label))
    (:then_1
      ;[0.15 0.15 0.15 0.5] DL to teleport enemy if they can't see Player
      (Utilities|FlowControl|Delay 5.0 :!label _label_2)
      (bind _outhit (Collision|LineTraceByChannel _returnvalue (Transformation|GetActorLocation _output_get) "TraceTypeQuery1" false 0 "ForDuration" true "(R=1.000000,G=0.000000,B=0.000000,A=1.000000)" "(R=0.000000,G=1.000000,B=0.000000,A=1.000000)" 3.0))
      (if (not (Utilities|Operators|EqualEqual :A (.location _outhit) :ErrorTolerance 0.0))
        (Transformation|SetActorLocation (.RandomLocation (AI|Navigation|GetRandomReachablePointinRadius (Transformation|GetActorLocation (Utilities|Array|Get(acopy) _outactors)) 3e+03 0 0)) false false)
        (goto _label_2)
        (else
          (goto _label_2))))))

(event Collision|EventHit
  (params (MyComp :type Primitive%20Component%20Object%20Reference) (Other :type Actor%20Object%20Reference) (OtherComp :type Primitive%20Component%20Object%20Reference) (bSelfMoved :type Boolean) (HitLocation :type Vector :default "0, 0, 0") (HitNormal :type Vector :default "0, 0, 0") (NormalImpulse :type Vector :default "0, 0, 0") (Hit :type Hit%20Result%20Structure%20%28by%20ref%29))
  ;[0.15 0.15 0.15 0.5] behavior based on HIT (other actor)
  (Development|PrintString "HIT SOMETHING")
  ;;[0.15 0.15 0.15 0.5] hit projectile
  (if (Utilities|ClassIsChildOf (Utilities|GetClass Other) "/Game/bluePrints/weapons/BP_baseFragment.BP_baseFragment_C")
    (Default|Damage/Heal (Variables|Default|GetBPC_HealthComponent))
    (Rendering|SetVisibility (Variables|Default|GetStun) true false)
    (bind _output_get (Variables|Default|SetstunExpiration (+ (Utilities|Time|GetGameTimeinSeconds) 2.0)))
    (Utilities|FlowControl|Delay 0.1 :!label _label)
    (if (<= _output_get (Utilities|Time|GetGameTimeinSeconds))
      (Rendering|SetVisibility (Variables|Default|GetStun) false false)
      (else
        (goto _label)))))

(event EventDealDmg/Heal
  (params (Damage/Heal :type Integer))
  (Default|Damage/Heal (Variables|Default|GetBPC_HealthComponent) Damage/Heal)
  (bind _returnvalue (Collision|LineTraceByChannel (Transformation|GetActorLocation) "0.000000,0.000000,-60.000000" "TraceTypeQuery1" false 0 "None"))
  (if _returnvalue
    (Utilities|FlowControl|Delay 0.2)
    (Character|LaunchCharacter "0.000000,0.000000,300.000000" false false)))

(fn ConstructionScript)