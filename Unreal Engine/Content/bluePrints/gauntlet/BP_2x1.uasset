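; BP_2x1 is a gauntlet platform that moves back and forth between its starting location and an EndPoint.
; On BeginPlay it records that location, binds movement to the level manager's GauntletActivated event and applies PlayRate to a timeline.
; The timeline lerps the relative location with sweep, and each finish flips MovingForward to alternate forward and reverse playback, looping the ping-pong.
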(event Custom|activateMoving
  ;[0.15 0.15 0.15 0.5] pingpongs between start and end position
  (if (Variables|Default|GetmovingForward) :!label _label
    (bind _platformpingpong (Timeline|Timeline PlayFromStart)
      (:Update
        (Transformation|SetActorRelativeLocation (Math|Vector|Lerp(Vector) (Variables|Default|GetstartPoint) (Variables|Default|GetendPoint) _platformpingpong) true))
      (:Finished
        (Variables|Default|SetmovingForward (not (Variables|Default|GetmovingForward)))
        (goto _label)))
    (else
      (Timeline|Timeline ReverseFromEnd))))

(event EventBeginPlay
  (Variables|Default|SetstartPoint (Transformation|GetActorLocation))
  (bind _returnvalue (Actor|GetActorOfClass "/Game/bluePrints/BP_levelManager.BP_levelManager_C"))
  (EventDispatchers|BindEventtoGauntletActivated _returnvalue (delegate Custom|activateMoving))
  (Components|Timeline|SetPlayRate (Variables|Default|GetTimeline) (Variables|Default|GetplayRate)))

(fn ConstructionScript)