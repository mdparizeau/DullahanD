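; BP_horizontalGuillotine is a gauntlet hazard whose middle post swings continuously back and forth between two points.
; On BeginPlay it binds its swing start to the level manager's gauntlet-activated event and applies a configurable timeline play rate.
; A timeline lerps the post between the start and end point locations with sweep enabled, flipping direction on each finish to loop.
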(event Custom|activateSwinging
  ;[0.15 0.15 0.15 0.5] alternates between swinging left and right continuously
  (if (Variables|Default|GethitForward) :!label _label
    (bind _alphamovement (Timeline|Timeline PlayFromStart)
      (:Update
        (Transformation|SetRelativeLocation (Variables|Default|GetmiddlePost) (Math|Vector|Lerp(Vector) (Variables|/Script/Engine.SceneComponent|GetRelativeLocation (Variables|Default|GetstartPoint)) (Variables|/Script/Engine.SceneComponent|GetRelativeLocation (Variables|Default|GetendPoint)) _alphamovement) true false))
      (:Finished
        (Variables|Default|SethitForward (not (Variables|Default|GethitForward)))
        (goto _label)))
    (else
      (Timeline|Timeline ReverseFromEnd))))

(event EventBeginPlay
  (bind _returnvalue (Actor|GetActorOfClass "/Game/bluePrints/BP_levelManager.BP_levelManager_C"))
  (EventDispatchers|BindEventtoGauntletActivated _returnvalue (delegate Custom|activateSwinging))
  (Components|Timeline|SetPlayRate (Variables|Default|GetTimeline) (Variables|Default|GetplayRate)))

(fn ConstructionScript)