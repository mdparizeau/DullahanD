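; BP_mageShot is a mage projectile that homes in on the player and destroys itself on impact.
; On BeginPlay it casts the player character to BP_FirstPersonCharacter and sets the first child of its capsule component as the ProjectileMovement homing target.
; Both overlap and hit events destroy the actor immediately, so a single collision removes the shot.
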(event Collision|EventHit
  (params (MyComp :type Primitive%20Component%20Object%20Reference) (Other :type Actor%20Object%20Reference) (OtherComp :type Primitive%20Component%20Object%20Reference) (bSelfMoved :type Boolean) (HitLocation :type Vector :default "0, 0, 0") (HitNormal :type Vector :default "0, 0, 0") (NormalImpulse :type Vector :default "0, 0, 0") (Hit :type Hit%20Result%20Structure%20%28by%20ref%29))
  ;[0.15 0.15 0.15 0.5] can change to Health Comp. to allow projs to be multiple hits (/collisions) to destroy
  (Actor|DestroyActor))

(event EventBeginPlay
  ;[0.15 0.15 0.15 0.5] Homes proj. toward Player
  (bind _asbp_first_person_character (Utilities|Casting|CastToBP_FirstPersonCharacter (Game|GetPlayerCharacter 0)))
  (bind _output_get (Variables|Default|SetAs%20BP%20First%20Person%20Character _asbp_first_person_character))
  (Variables|/Script/Engine.ProjectileMovementComponent|SetHomingTargetComponent (Variables|Default|GetProjectileMovement) (Components|GetChildComponent (Variables|/Script/Engine.Character|GetCapsuleComponent _output_get) 0)))

(event Collision|EventActorBeginOverlap
  (params (OtherActor :type Actor%20Object%20Reference))
  ;[0.15 0.15 0.15 0.5] can change to Health Comp. to allow projs to be multiple hits (/collisions) to destroy
  (Actor|DestroyActor))

(fn ConstructionScript
  (|CallParentFunction))