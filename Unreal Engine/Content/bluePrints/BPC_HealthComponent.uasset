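; BPC_HealthComponent is an actor component that tracks health for its owner and handles death.
; Health starts at the maximum on BeginPlay, and one Damage/Heal event subtracts a signed amount, clamped between zero and the maximum.
; At zero it prints a debug message and destroys the owner only if it derives from BP_baseEnemy.
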(event Custom|Damage/Heal
  (params (Amount :type Integer))
  (bind _returnvalue (Components|GetOwner))
  (bind _output_get (Variables|Default|SetCurrent%20Health (Math|Integer|Clamp(Integer) (- (Variables|Default|GetCurrent%20Health) Amount) 0 (Variables|Default|GetMax%20Health))))
  (if (<= _output_get 0)
    (Development|PrintString "die")
    (if (Utilities|ClassIsChildOf (Utilities|GetClass _returnvalue) "/Game/bluePrints/BP_baseEnemy.BP_baseEnemy_C")
      (Actor|DestroyActor _returnvalue))))

(event EventBeginPlay
  (Variables|Default|SetCurrent%20Health (Variables|Default|GetMax%20Health)))