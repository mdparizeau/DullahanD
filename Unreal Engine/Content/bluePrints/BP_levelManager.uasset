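; Level manager Blueprint that owns the dialogue HUD, finds the area or building nearest the player, and fires the gauntlet for one specific section.
; Branching NPC dialogue, with skull reactions, walks a flattened three-way node tree, computing each index from depth, choice and previous index.
; It sends lines to WBP_HUD, then enables non-empty player options on line completion or ends the dialogue.
; An older line-array dialogue path remains, partly disconnected.
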(event Custom|outputDialogueToScreen
  (params (dialogueLine :type String))
  (Class|BPIDialogueLine|DialogueLine(Message) (Variables|NEW|GetHUD%20Reference) dialogueLine))

(event Custom|weDone
  ;[0.15 0.15 0.15 0.5] resets all dialogue variables and signals for UI to do the same
  (Class|BPIDialogueOverride|DialogueOverride(Message) (Variables|NEW|GetHUD%20Reference) true false)
  (Variables|Default|SetisDisengaged true)
  (Variables|Default|SetdialogueOptions "")
  (Variables|Default|SetlineNumber 0)
  ;;[0 1 0.005287 0.5] MIGHT STILL NEED THIS
  (Variables|Default|SetOption%20Number 0)
  (Class|BPIEndInteraction|EndInteraction(Message) (Variables|NEW|GetPlayer%20Reference) (Variables|Default|GetcurrentKey))
  (Widget|SetVisibility (Variables|NEW|GetHUD%20Reference) "Collapsed")
  (Class|BPILineFinished|LineFinished(Message) (Variables|NEW|GetPlayer%20Reference)))

(event Custom|Append%20Lines%20to%20Print
  (params (SR->Player :type String) (NPC :type String) (SR->NPC :type String) (Player%20Op.%201 :type String) (Player%20Op.%202 :type String) (Player%20Op.%203 :type String) (Skill%20Required :type ENUM_PlayerSkills%20Enum :default "NewEnumerator0"))
  (Development|PrintString "start NPC lines")
  (if (Utilities|Enum|Equal(Enum) SR->Player "")
    _
    (else
      (CallFunction|PrintLine (Utilities|String|Append "<speaker>Skull reaction to player:</> " SR->Player))))
  (if (Utilities|Enum|Equal(Enum) NPC "")
    _
    (else
      (CallFunction|PrintLine (Utilities|String|Append "<speaker>NPC: </> " NPC))))
  (if (Utilities|Enum|Equal(Enum) SR->NPC "")
    _
    (else
      (CallFunction|PrintLine (Utilities|String|Append "<speaker>Skull reaction to NPC: </> " SR->NPC))))
  (CallFunction|DisplayandEnablePlayerOptions Player%20Op.%201 Player%20Op.%202 Player%20Op.%203 Skill%20Required)
  (Development|PrintString "finish NPC lines"))

(event Custom|Display%20and%20Enable%20Player%20Options
  (params (Player%20Op.%201 :type String) (Player%20Op.%202 :type String) (Player%20Op.%203 :type String) (Skill%20Required :type ENUM_PlayerSkills%20Enum :default "NewEnumerator0"))
  ;[0.15 0.15 0.15 0.5] Swap order of Options and printing to support conditionals
  (CallFunction|SetandDisplayOptionAvailability Player%20Op.%201 Player%20Op.%202 Player%20Op.%203))

(event Custom|Set%20and%20Display%20Option%20Availability
  (params (Player%20Op.%201 :type String) (Player%20Op.%202 :type String) (Player%20Op.%203 :type String))
  ;[0.15 0.15 0.15 0.5] Sets and Displays Player's Options' availability based on them being empty or not
  (if (Utilities|Enum|Equal(Enum) Player%20Op.%201 "")
    (Variables|NEW|SetIs%20Op_%201%20Available false)
    (else
      (Variables|NEW|SetIs%20Op_%201%20Available true)
      (Variables|NEW|SetplayerOptions (Utilities|String|Append (Variables|NEW|GetplayerOptions) "1.) " Player%20Op.%201 " 
"))
      (if (Utilities|Enum|Equal(Enum) Player%20Op.%202 "")
        (Variables|NEW|SetIs%20Op_%202%20Available false)
        (else
          (Variables|NEW|SetIs%20Op_%202%20Available true)
          (Variables|NEW|SetplayerOptions (Utilities|String|Append (Variables|NEW|GetplayerOptions) "2.) " Player%20Op.%202 " 
"))))
      (if (Utilities|Enum|Equal(Enum) Player%20Op.%203 "")
        (Variables|NEW|SetIs%20Op_%203%20Available false)
        (else
          (Variables|NEW|SetIs%20Op_%203%20Available true)
          (bind _output_get (Variables|NEW|SetplayerOptions (Utilities|String|Append (Variables|NEW|GetplayerOptions) "3.) " Player%20Op.%203)))))
      (CallFunction|PrintLine _output_get))))

(event Custom|Print%20Line
  (params (lineToPrint :type String))
  ;[0.15 0.15 0.15 0.5] Send line to print to WBP_HUD
  (Class|BPIDialogueLine|DialogueLine(Message) (Variables|NEW|GetHUD%20Reference) lineToPrint))

(event Custom|End%20Dialogue
  ;[0 0.15 0.0066 0.5] Reset variables for next dialogue
  (Variables|NEW|SetdialogueLevel -1)
  (Variables|NEW|SetnodeIndex 0)
  (Variables|NEW|SetIs%20Op_%201%20Available false)
  (Variables|NEW|SetIs%20Op_%202%20Available false)
  (Variables|NEW|SetIs%20Op_%203%20Available false)
  (Variables|NEW|SetplayerOptions "")
  (Widget|SetVisibility (Variables|NEW|GetHUD%20Reference) "Collapsed"))

(event EventNPCInteraction
  (params (E_dialogueKey :type ENUM_dialogueInteractions%20Enum :default "NewEnumerator0") (playerReference :type BP%20First%20Person%20Character%20Object%20Reference))
  (bind _e_dialogueinteractions (Variables|Default|GetE_dialogueInteractions))
  (bind _option_number (Variables|Default|GetOption%20Number))
  (bind _linenumber (Variables|Default|GetlineNumber))
  (bind _value (Utilities|Map|Find _e_dialogueinteractions E_dialogueKey))
  (bind _dialogue_lines (Utilities|Struct|Breakdialogue _value))
  (bind _output (Utilities|Array|Get(acopy) _dialogue_lines _linenumber))
  (bind (_player_branch _npc_branch _skull_npc_branch _skull_player_branch) (Utilities|Struct|Breakbranches _output))
  (bind _output_2 (Utilities|Array|Get(acopy) _npc_branch _option_number))
  (bind _output_3 (Utilities|Array|Get(acopy) _skull_npc_branch _option_number))
  (bind _returnvalue (Utilities|String|Append "<speaker>NPC: </>" _output_2))
  (bind _returnvalue_2 (Utilities|String|Append "<speaker>Skull reaction to NPC: </>" _output_3))
  (Variables|Default|SetcurrentKey E_dialogueKey)
  (Variables|Default|SetisDisengaged false)
  (Widget|SetVisibility (Variables|NEW|GetHUD%20Reference) "Visible")
  (Variables|Default|SetcurrentDialogue _dialogue_lines)
  (if (not (Variables|Default|GetisDisengaged))
    (CallFunction|OutputDialoguetoScreen _returnvalue)
    (Development|PrintString _returnvalue)
    (if (not (Variables|Default|GetisDisengaged))
      (CallFunction|OutputDialoguetoScreen _returnvalue_2)
      (Development|PrintString _returnvalue_2)
      (bind _result (Math|Integer|IncrementInt (Variables|Default|GetlineNumber))
        (:%20%20
          (if (>= _result (Utilities|Array|Length (Variables|Default|GetcurrentDialogue)))
            (Variables|Default|SetisDialogueCompleted true)
            (else
              (Variables|Default|Setcurrent_skull_player_reaction (.skull_player_branch (Utilities|Struct|Breakbranches (Utilities|Array|Get(acopy) (Variables|Default|GetcurrentDialogue) _result))))
              (for (_array_element _array_index) (.player_branch (Utilities|Struct|Breakbranches (Utilities|Array|Get(acopy) (Variables|Default|GetcurrentDialogue) _result)))
                (bind _output_get (Variables|Default|SetdialogueOptions (Utilities|String|Append (Variables|Default|GetdialogueOptions) (Utilities|String|Append "<speaker>Option </>" (Utilities|String|ToString(Integer) (+ _array_index 1)) "<speaker>: </>" _array_element " 
"))))
                (Development|PrintString (Utilities|String|Append "<speaker>Option </>" (Utilities|String|ToString(Integer) (+ _array_index 1)) "<speaker>: </>" _array_element " 
")))
              (if (not (Variables|Default|GetisDisengaged))
                (CallFunction|OutputDialoguetoScreen _output_get)
                (Variables|Default|SetdialogueOptions "")))))))))

(event EventLineFinished
  ;[0.15 0.15 0.15 0.5] Swap order of Options and printing to support conditionals
  (Class|BPIAllowPlayerInput|EnablePlayerInput(Message) (Variables|NEW|GetPlayer%20Reference) (stale Custom|Display%20and%20Enable%20Player%20Options Skill%20Required) (Variables|NEW|GetIs%20Op_%201%20Available) (Variables|NEW|GetIs%20Op_%202%20Available) (Variables|NEW|GetIs%20Op_%203%20Available))
  (Development|PrintString "AVAILABILITY SENT")
  (if (not (Variables|NEW|GetIs%20Op_%201%20Available))
    (CallFunction|EndDialogue)))

(event EventStartDialogue
  (params (dialogueNodes :type Array%20of%20Dialogue%20Node%20Structures) (playerReference :type BP%20First%20Person%20Character%20Object%20Reference))
  (bind _output (Utilities|Array|Get(acopy) dialogueNodes))
  (bind (_sr__player _npc _sr__npc _playerop1 _playerop2 _playerop3 _skillrequired) (Utilities|Struct|BreakdialogueNode _output))
  (Variables|NEW|SetNEW_currentDialogue dialogueNodes)
  (Variables|NEW|SetPlayer%20Reference playerReference)
  (CallFunction|AppendLinestoPrint _sr__player _npc _sr__npc _playerop1 _playerop2 _playerop3 _skillrequired)
  (Widget|SetVisibility (Variables|NEW|GetHUD%20Reference) "Visible"))

(event EventBeginPlay
  (bind _returnvalue (UserInterface|CreateWidget "/Game/bluePrints/UI/WBP_HUD.WBP_HUD_C"))
  (bind _output_get (Variables|NEW|SetHUD%20Reference _returnvalue))
  (UserInterface|Viewport|AddtoViewport _output_get 0)
  (Widget|SetVisibility (Variables|NEW|GetHUD%20Reference) "Collapsed"))

(event EventCheckSection
  (params (playerLocation :type Vector :default "0, 0, 0") (isArea :type Boolean))
  ;[0.15 0.15 0.15 0.5] Checks if area or building, then the distance between the player and all sectionAreas/Buildings; sets and displays closest sectionArea/Building
  (if isArea
    (bind _output_get (Variables|Default|SetE_sectionObjects_toUse (Variables|Default|GetE_sectionObjects_areas)))
    (else
      (Variables|Default|SetE_sectionObjects_toUse (Variables|Default|GetE_sectionObjects_buildings))))
  (bind (_keypin _valuepin) (Utilities|Map|ForEachLoop(Map) _output_get)
    (:then
      (if (< (Math|Vector|Distance(Vector) (Transformation|GetActorLocation _valuepin) playerLocation) (Variables|Default|GetclosestSection_distance))
        (bind _output_get_2 (Variables|Default|SetE_closestSection _keypin))
        (Variables|Default|SetclosestSection_distance (Math|Vector|Distance(Vector) (Transformation|GetActorLocation _valuepin) playerLocation))))
    (:CompletedPin
      (Development|PrintString (.Value (Utilities|Map|Find (Variables|Default|GetE_sectionNames) _output_get_2)))
      (if (Utilities|Enum|Equal(Enum) _output_get_2 "NewEnumerator4")
        (Default|CallGauntletActivated)))))

(event EventDialogueOverride
  (params (disengaged :type Boolean) (finishLine :type Boolean))
  ;[0.15 0.15 0.15 0.5] manual disengagement
  (if disengaged
    (CallFunction|WeDone)
    (else
      (Class|BPIDialogueOverride|DialogueOverride(Message) (Variables|NEW|GetHUD%20Reference) false finishLine))))

(event EventContinueDialogue
  (params (optionChoice :type Integer))
  (Variables|NEW|SetplayerOptions "")
  (bind _result (Math|Integer|IncrementInt (Variables|NEW|GetdialogueLevel))
    (:%20%20
      (bind _newnodeindex (CallFunction|CalculateNodeIndex _result optionChoice (Variables|NEW|GetnodeIndex)))
      (bind _output_get (Variables|NEW|SetnodeIndex _newnodeindex))
      (CallFunction|AppendLinestoPrint (.SR->Player (Utilities|Struct|BreakdialogueNode (Utilities|Array|Get(acopy) (Variables|NEW|GetNEW_currentDialogue) _output_get))) (.NPC (Utilities|Struct|BreakdialogueNode (Utilities|Array|Get(acopy) (Variables|NEW|GetNEW_currentDialogue) _output_get))) (.SR->NPC (Utilities|Struct|BreakdialogueNode (Utilities|Array|Get(acopy) (Variables|NEW|GetNEW_currentDialogue) _output_get))) (.PlayerOp1 (Utilities|Struct|BreakdialogueNode (Utilities|Array|Get(acopy) (Variables|NEW|GetNEW_currentDialogue) _output_get))) (.PlayerOp2 (Utilities|Struct|BreakdialogueNode (Utilities|Array|Get(acopy) (Variables|NEW|GetNEW_currentDialogue) _output_get))) (.PlayerOp3 (Utilities|Struct|BreakdialogueNode (Utilities|Array|Get(acopy) (Variables|NEW|GetNEW_currentDialogue) _output_get))) (.SkillRequired (Utilities|Struct|BreakdialogueNode (Utilities|Array|Get(acopy) (Variables|NEW|GetNEW_currentDialogue) _output_get)))))))

(fn ConstructionScript)

(fn CalculateNodeIndex
  (params (Dialogue%20Level :type Integer) (Player%20Choice :type Integer) (previousNodeIndex :type Integer))
  (return (+ (* (Math|Float|Power 3.0 (Math|Conversions|ToFloat(Integer) Dialogue%20Level)) Player%20Choice) previousNodeIndex)))